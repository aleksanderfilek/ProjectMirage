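; BP_StreamingManager loads and unloads groups of streaming levels by a LevelId.
; Stream looks up the LevelId row in StreamingTable and asynchronously loads each listed level that is not yet loaded, making it visible afterward.
; Unstream reads the same row and unloads each loaded level without blocking.
; Init and the construction script only call their parent versions.
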(event `Stream`
  (params (LevelId :type Name))
  (bind _returnvalue (`|GetDataTableRow` "/Game/Blueprints/Streaming/StreamingTable.StreamingTable" LevelId)
    (:`then`
      (for _array_element (`.Levels_7_8E1F5A0641E84E4D40E23AB3DADD5DA9` (break `/Game/Blueprints/Streaming/StreamingLevelsRow` _returnvalue))
        (if (not (`LevelStreaming.IsLevelLoaded` (`GameplayStatics.GetStreamingLevel` _array_element)))
          (`GameplayStatics.LoadStreamLevel` _array_element true))))))

(event `Unstream`
  (params (LevelId :type Name))
  (bind _returnvalue (`|GetDataTableRow` "/Game/Blueprints/Streaming/StreamingTable.StreamingTable" LevelId)
    (:`then`
      (for _array_element (`.Levels_7_8E1F5A0641E84E4D40E23AB3DADD5DA9` (break `/Game/Blueprints/Streaming/StreamingLevelsRow` _returnvalue))
        (if (`LevelStreaming.IsLevelLoaded` (`GameplayStatics.GetStreamingLevel` _array_element))
          (`GameplayStatics.UnloadStreamLevel` _array_element))))))

(fn `Init`
  (`parent.Init`))

(fn `UserConstructionScript`
  (`parent.UserConstructionScript`))