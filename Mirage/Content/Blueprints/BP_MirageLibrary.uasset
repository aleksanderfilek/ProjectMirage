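; BP_MirageLibrary is a helper library of global getters for the Mirage game's core framework objects.
; It returns the cast game mode, the player controller at index 0, and the quest and streaming managers.
; Both managers are looked up by class in the game mode's Managers map, so the game mode acts as their registry.
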(fn `GetMirageGameMode`
  (returns (GameMode :type "/Game/Blueprints/BP_MirageGameMode Object Reference"))
  (bind _asbp_mirage_game_mode (cast `/Game/Blueprints/BP_MirageGameMode` (`GameplayStatics.GetGameMode` (`local.__WorldContext`))))
  (return _asbp_mirage_game_mode))

(fn `GetMiragePlayerController`
  (returns (PlayerController :type "/Game/Blueprints/BP_MiragePlayerController Object Reference"))
  (bind _asbp_mirage_player_controller (cast `/Game/Blueprints/BP_MiragePlayerController` (`GameplayStatics.GetPlayerController` (`local.__WorldContext`))))
  (return _asbp_mirage_player_controller))

(fn `GetQuestManager`
  (returns (QuestManager :type "/Game/Blueprints/Quest/BP_QuestManager Object Reference"))
  (bind _asbp_mirage_game_mode (cast `/Game/Blueprints/BP_MirageGameMode` (`GameplayStatics.GetGameMode` (`local.__WorldContext`))))
  (bind _asbp_quest_manager (cast `/Game/Blueprints/Quest/BP_QuestManager` (`BlueprintMapLibrary.Map_Find` (`/Game/Blueprints/BP_MirageGameMode.Managers` _asbp_mirage_game_mode) "/Game/Blueprints/Quest/BP_QuestManager.BP_QuestManager_C")))
  (return _asbp_quest_manager))

(fn `GetStreamingManager`
  (returns (StreamingManager :type "/Game/Blueprints/Streaming/BP_StreamingManager Object Reference"))
  (bind _asbp_mirage_game_mode (cast `/Game/Blueprints/BP_MirageGameMode` (`GameplayStatics.GetGameMode` (`local.__WorldContext`))))
  (bind _asbp_streaming_manager (cast `/Game/Blueprints/Streaming/BP_StreamingManager` (`BlueprintMapLibrary.Map_Find` (`/Game/Blueprints/BP_MirageGameMode.Managers` _asbp_mirage_game_mode) "/Game/Blueprints/Streaming/BP_StreamingManager.BP_StreamingManager_C")))
  (return _asbp_streaming_manager))