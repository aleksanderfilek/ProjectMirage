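; BP_HintManager is a manager Blueprint that shows and hides on-screen hints in the game's HUD.
; On Init it calls the parent and caches the UIHintWB widget from the Mirage HUD.
; Show converts a hint type enum to its name and passes it to that widget, and Hide tells the widget to hide.
; The event graph has no active logic, so all behavior runs through these functions.
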(fn `Hide`
  (`/Game/Blueprints/Widgets/UI_Hint_WB.Hide` (`self.HintWB`)))

(fn `Init`
  (`parent.Init`)
  (set `self.HintWB` (`/Game/Blueprints/Widgets/UI_Hud.UI_Hint_WB` (`/Game/Blueprints/BP_MirageLibrary.GetMirageHud`))))

(fn `Show`
  (params (Type :type "/Game/Blueprints/Hint/HintType Enum" :default "NewEnumerator0"))
  (`/Game/Blueprints/Widgets/UI_Hint_WB.Show` (`self.HintWB`) (`|GetEnumeratorName` Type)))

(fn `UserConstructionScript`
  (`parent.UserConstructionScript`))