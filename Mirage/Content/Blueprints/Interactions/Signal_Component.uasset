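; Signal_Component is an actor component that passes a value between interaction actors through configured send and receive lists.
; At BeginPlay it registers itself in the SendSignalsToList of each component in its RecieveSignalsFromList, so links can be declared from the receiving side.
; SendSignal(s) fires OnSignalRecieved on every target, passing itself and the value.
; A macro resolves list entries, stored as actor plus component index, allowing several signal components per actor.
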(event `self.ReceiveBeginPlay`
  (bind _returnvalue (`self.GetOwner`))
  (bind _output (`self.For Each Component in Array` (`self.Recieve Signals From List`))
    (:`LoopBody`
      (`KismetArrayLibrary.Array_AddUnique` (`/Game/Blueprints/Interactions/Signal_Component.Send Signals To List` _output) (make `/Game/Blueprints/Interactions/SignalComponentIdentifier` _returnvalue (`KismetArrayLibrary.Array_Find` (`Actor.K2_GetComponentsByClass` _returnvalue "Signal_Component_C") self))))))

(event `Send Signal(s)`
  (params (Value :type Integer))
  (bind _output (`self.For Each Component in Array` (`self.Send Signals To List`))
    (:`LoopBody`
      (`self.OnSignalRecieved` _output self Value))))