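; Draggable lever interaction that sends a signal when pulled past an activation threshold.
; A child-actor drag collision reports drag deltas, which pitch the lever within a symmetric angle limit.
; Each step combines the vertical drag sign with the length of the collision's up vector projected onto the delta, scaled by speed.
; Dropping below the threshold fires the SignalComponent once, re-arming when a drag brings it back.
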(event `self.ReceiveBeginPlay`
  (bind _asdraggable_collision (cast `/Game/Blueprints/Interactions/Interactions/DraggableCollision` (`ChildActorComponent.ChildActor` (`self.DraggableCollision`))))
  (add `/Game/Blueprints/Interactions/Interactions/DraggableCollision.OnDragDelta` _asdraggable_collision (delegate `OnDragDelta`)))

(event `OnDragDelta`
  (params (Delta :type "Vector Structure") (DeltaTime :type "Float (double-precision)"))
  (bind _maxangle (`self.MaxAngle`))
  (bind _returnvalue (`KismetMathLibrary.ClampAngle` (+ (* (* (`KismetMathLibrary.SignOfFloat` (.z Delta)) (`KismetMathLibrary.VSize` (`KismetMathLibrary.ProjectVectorOnToVector` (`SceneComponent.GetUpVector` (`self.DraggableCollision`)) Delta))) (`self.Speed`)) (.pitch (.rotation (`SceneComponent.GetRelativeTransform` (`self.Lever`))))) (* _maxangle -1.0) _maxangle))
  (`SceneComponent.K2_SetRelativeRotation` (`self.Lever`) (`KismetMathLibrary.MakeRotator` 0.0 _returnvalue) false false)
  (if (< _returnvalue (`self.ActivationThreshold`))
    (`/Engine/EditorBlueprintResources/StandardMacros.DoOnce` false :!label _label
      (:`Completed`
        (`/Game/Blueprints/Interactions/Signal_Component.Send Signal(s)` (`self.Signal_Component`) 1)
        (`KismetSystemLibrary.PrintString` "Lever Activated")))
    (else
      (set `self.Active` false)
      (goto _label :!via `Reset`))))

(fn `UserConstructionScript`)