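; Physics door variant that can be locked and unlocked remotely through its Signal Component.
; Signal 0 locks it, disables interaction on the draggable knob child actor and, if the door is simulating physics, shoves it shut with an impulse along the knob's right vector.
; Signal 1 unlocks it and restores knob interaction.
; The construction script applies the initial Locked state to the knob.
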(event `self.Signal_Component.OnSignalRecieved`
  (params (`From Component` :type "/Game/Blueprints/Interactions/Signal_Component Object Reference") (Value :type Integer))
  (bind _door (`self.Door`))
  (bind _interactions_component (`/Game/Blueprints/Interactions/Interactions/DraggableCollision.Interactions_Component` (cast `/Game/Blueprints/Interactions/Interactions/DraggableCollision` (`ChildActorComponent.ChildActor` (`self.Knob`)) :!pure true)))
  (switch `int` Value
    (:`0`
      (if (not (`self.Locked`))
        (set `self.Locked` true)
        (`KismetSystemLibrary.PrintString` "Door Closed")
        (`/Game/Blueprints/Interactions/Interactions_Component.SetCanBeInteractedWith` _interactions_component false)
        ;[1 1 1] Shut the door
        (if (`SceneComponent.IsSimulatingPhysics` _door "None")
          (`PrimitiveComponent.AddImpulse` _door (* (`SceneComponent.GetRightVector` (`self.Knob`)) 1 400000.0) "None" false))))
    (:`1`
      (if (`self.Locked`)
        (set `self.Locked` false)
        (`KismetSystemLibrary.PrintString` "Door Opened")
        (`/Game/Blueprints/Interactions/Interactions_Component.SetCanBeInteractedWith` _interactions_component true)))))

(fn `UserConstructionScript`
  (`parent.UserConstructionScript`)
  (bind _asdraggable_collision (cast `/Game/Blueprints/Interactions/Interactions/DraggableCollision` (`ChildActorComponent.ChildActor` (`self.Knob`))))
  (`/Game/Blueprints/Interactions/Interactions_Component.SetCanBeInteractedWith` (`/Game/Blueprints/Interactions/Interactions/DraggableCollision.Interactions_Component` _asdraggable_collision) (not (`self.Locked`))))