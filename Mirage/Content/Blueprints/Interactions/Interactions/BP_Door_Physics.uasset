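; Physics-driven interactive door that the player opens by dragging its knob, a draggable collision child actor.
; Starting a drag enables physics simulation on the door, and each drag delta applies a time-scaled impulse to push it.
; Tick tracks the physics constraint's Swing1 angle; when its sign flips while the knob is not held, the door stops simulating and snaps back to closed.
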(event `self.ReceiveBeginPlay`
  ;[1 1 1] Bind Knob Events
  (bind _asdraggable_collision (cast `/Game/Blueprints/Interactions/Interactions/DraggableCollision` (`ChildActorComponent.ChildActor` (`self.Knob`))))
  (add `/Game/Blueprints/Interactions/Interactions/DraggableCollision.OnDragDelta` _asdraggable_collision (delegate `On Knob Dragged`))
  (add `/Game/Blueprints/Interactions/Interactions/DraggableCollision.OnDragStarted` _asdraggable_collision (delegate `Open Door`))
  (add `/Game/Blueprints/Interactions/Interactions/DraggableCollision.OnDragEnded` _asdraggable_collision (delegate `Stop Dragging Knob`)))

(event `self.ReceiveTick`
  (params (DeltaSeconds :type "Float (single-precision)"))
  (`|ExecutionSequence`
    (:`then_0`
      ;[1 1 1] If the door passes through frame without holding, close and reset it
      (if (and (< (* (`PhysicsConstraintComponent.GetCurrentSwing1` (`self.PhysicsConstraint`)) (`self.Tracked Swing`)) 0.0) (not (`self.IsBeingDragged`)))
        (`self.CloseDoor`)))
    (:`then_1`
      ;[1 1 1] Track Swing
      (set `self.Tracked Swing` (`PhysicsConstraintComponent.GetCurrentSwing1` (`self.PhysicsConstraint`))))))

(event `On Knob Dragged`
  (params (Delta :type "Vector Structure") (DeltaTime :type "Float (double-precision)"))
  ;[1 1 1] Every Tick Push Door towards Component
  (if (`SceneComponent.IsSimulatingPhysics` (`self.Door`) "None")
    (`PrimitiveComponent.AddImpulse` (`self.Door`) (* Delta (* DeltaTime 3000.0)) "None" false)))

(event `CloseDoor`
  (bind _door (`self.Door`))
  ;[1 1 1] Cloe and reset door
  (`PrimitiveComponent.SetSimulatePhysics` _door false)
  (`SceneComponent.K2_SetRelativeRotation` :`self` _door))

(event `Open Door`
  ;[1 1 1] Start Dragging
  (`PrimitiveComponent.SetSimulatePhysics` (`self.Door`) true)
  (set `self.IsBeingDragged` true))

(event `Stop Dragging Knob`
  (set `self.IsBeingDragged` false))

(fn `UserConstructionScript`)