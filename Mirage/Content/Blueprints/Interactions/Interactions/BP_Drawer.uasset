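; BP_Drawer is an interactable physics drawer that slides open and closed when its knob is dragged.
; The knob's DraggableCollision child actor enables physics when a drag starts, then drives impulses from the drag delta projected onto the drawer's right vector.
; Tick limits travel between the start position and Max along world Y, briefly disabling physics to snap the drawer back to the limit.
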(event `self.ReceiveBeginPlay`
  (set `self.StartLocation` (`SceneComponent.K2_GetComponentLocation` (`self.Drawer`)))
  (bind _asdraggable_collision (cast `/Game/Blueprints/Interactions/Interactions/DraggableCollision` (`ChildActorComponent.ChildActor` (`self.Knob`))))
  (add `/Game/Blueprints/Interactions/Interactions/DraggableCollision.OnDragDelta` _asdraggable_collision (delegate `OnKnobDrag`))
  (add `/Game/Blueprints/Interactions/Interactions/DraggableCollision.OnDragStarted` _asdraggable_collision (delegate `OnKnobDragStart`))
  (add `/Game/Blueprints/Interactions/Interactions/DraggableCollision.OnDragEnded` _asdraggable_collision (delegate `OnKnobDragEnded`)))

(event `self.ReceiveTick`
  (params (DeltaSeconds :type "Float (single-precision)"))
  (bind _drawer (`self.Drawer`))
  (bind _drawer_2 (`self.Drawer`))
  (bind _y (.y (- (`self.StartLocation`) (`SceneComponent.K2_GetComponentLocation` (`self.Drawer`)))))
  (if (< _y 0.0)
    (`PrimitiveComponent.SetSimulatePhysics` _drawer false)
    (`SceneComponent.K2_SetWorldLocation` _drawer (`self.StartLocation`) false false)
    (`PrimitiveComponent.SetSimulatePhysics` (`self.Drawer`) true)
    (elif (> _y (`self.Max`))
      (`PrimitiveComponent.SetSimulatePhysics` _drawer_2 false)
      (`SceneComponent.K2_SetWorldLocation` _drawer_2 (+ (`self.StartLocation`) (`KismetMathLibrary.MakeVector` 0.0 (* (`self.Max`) -1.0))) false false)
      (`PrimitiveComponent.SetSimulatePhysics` (`self.Drawer`) true))))

(event `OnKnobDrag`
  (params (Delta :type "Vector Structure") (DeltaTime :type "Float (double-precision)"))
  (if (`SceneComponent.IsSimulatingPhysics` (`self.Drawer`) "None")
    (`PrimitiveComponent.AddImpulse` (`self.Drawer`) (* (`KismetMathLibrary.ProjectVectorOnToVector` Delta (`SceneComponent.GetRightVector` (`self.Drawer`))) (* DeltaTime 1000.0)) "None" false)))

(event `OnKnobDragStart`
  (`PrimitiveComponent.SetSimulatePhysics` (`self.Drawer`) true)
  (set `self.IsBeingDragged` true))

(event `OnKnobDragEnded`
  (set `self.IsBeingDragged` false))

(fn `UserConstructionScript`)