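; BP_Doors is an interactable door that the player swings by dragging while the interaction is held.
; Interaction start caches the Mirage character and sets its drag point to TargetLocation; interaction end clears the reference.
; While that reference is valid, Tick derives a signed yaw from the drag point against the root's backward and right vectors, clamped symmetrically by MaxAngle.
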(event `self.ReceiveTick`
  (params (DeltaSeconds :type "Float (single-precision)"))
  (bind _defaultsceneroot (`self.DefaultSceneRoot`))
  (bind _maxangle (`self.MaxAngle`))
  (bind _returnvalue (- (`/Game/Blueprints/Characters/BP_MirageDefaultCharacter.GetDragPointLocation` (`self.CharacterRef`)) (`SceneComponent.K2_GetComponentLocation` (`self.Door`))))
  (`/Engine/EditorBlueprintResources/StandardMacros.IsValid` (`self.CharacterRef`)
    (:`Is Valid`
      (`SceneComponent.K2_SetRelativeRotation` (`self.Door`) (`KismetMathLibrary.MakeRotator` 0.0 0.0 (`KismetMathLibrary.ClampAngle` (* (`KismetMathLibrary.SelectInt` -1 1 (<= (`KismetMathLibrary.DegAcos` (`KismetMathLibrary.Vector_CosineAngle2D` (`SceneComponent.GetRightVector` _defaultsceneroot) _returnvalue)) 90.0)) (`KismetMathLibrary.DegAcos` (`KismetMathLibrary.Vector_CosineAngle2D` (* (`SceneComponent.GetForwardVector` _defaultsceneroot) -1.0) _returnvalue))) (* -1 _maxangle) _maxangle)) false false))))

(event `self.Interactions_Component.OnInteractStart`
  (bind _asbp_mirage_default_character (cast `/Game/Blueprints/Characters/BP_MirageDefaultCharacter` (`/Game/Blueprints/BP_MiragePlayerController.CharacterPawnRef` (`/Game/Blueprints/BP_MirageLibrary.GetMiragePlayerController`))))
  (bind _output_get (set `self.CharacterRef` _asbp_mirage_default_character))
  (`/Game/Blueprints/Characters/BP_MirageDefaultCharacter.SetDragPointLocation` _output_get (`/Game/Blueprints/Characters/BP_MirageDefaultCharacter.TargetLocation` _output_get)))

(event `self.Interactions_Component.OnInteractEnd`
  (set `self.CharacterRef` null))

(fn `UserConstructionScript`)