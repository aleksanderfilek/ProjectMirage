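; Interaction component that tracks whether something can be, or is being, interacted with and announces when interaction starts and ends.
; Interact and StopInteracting flip the IsBeingInteractedWith state only while interaction is allowed, calling OnInteractStart or OnInteractEnd on each change.
; SetCanBeInteractedWith sets that permission and, when set to true, clears any active interaction without calling OnInteractEnd.
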(event `Event Interact`
  (if (`self.IsBeingInteractedWith`)
    _
    (elif (`self.Can Be Interacted With`)
      (set `self.IsBeingInteractedWith` true)
      (`self.OnInteractStart`))))

(event `Event Stop Interacting`
  (if (`self.IsBeingInteractedWith`)
    (if (`self.Can Be Interacted With`)
      (set `self.IsBeingInteractedWith` false)
      (`self.OnInteractEnd`))))

(fn `SetCanBeInteractedWith`
  (params (`Input Value` :type Boolean))
  (bind _output_get (set `self.Can Be Interacted With` `Input Value`))
  (if _output_get
    (if (`self.IsBeingInteractedWith`)
      (set `self.IsBeingInteractedWith` false))))