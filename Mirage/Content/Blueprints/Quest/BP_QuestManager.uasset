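; Quest manager that keeps the game's registered quests and named facts, and serves as a front for dialogue and story block requests.
; Init fetches the dialogue manager from the Mirage game mode's Managers map and caches it along with the hint manager.
; Dialogue and story block calls forward to the dialogue manager, while quests register without duplicates and facts are stored and read by name.
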(fn `AddFact`
  (params (Name :type Name) (Value :type Boolean))
  (`BlueprintMapLibrary.Map_Add` (`self.Facts`) Name Value))

(fn `GetFactValue`
  (params (Name :type Name))
  (returns (Value :type Boolean))
  (return (`BlueprintMapLibrary.Map_Find` (`self.Facts`) Name)))

(fn `Init`
  (`parent.Init`)
  (bind _asbp_dialogue_manager (cast `/Game/Blueprints/Quest/Dialogues/BP_DialogueManager` (`BlueprintMapLibrary.Map_Find` (`/Game/Blueprints/BP_MirageGameMode.Managers` (`/Game/Blueprints/BP_MirageLibrary.GetMirageGameMode`)) "/Game/Blueprints/Quest/Dialogues/BP_DialogueManager.BP_DialogueManager_C")))
  (set `self.DialogueManagerRef` _asbp_dialogue_manager)
  (set `self.HintManagerRef` (`/Game/Blueprints/BP_MirageLibrary.GetHintManager`)))

(fn `IsDialoguePlaying`
  (returns (Playing :type Boolean))
  (return (`/Game/Blueprints/Quest/Dialogues/BP_DialogueManager.IsPlaying` (`self.DialogueManagerRef`))))

(fn `IsStoryBlockActive`
  (returns (Active :type Boolean))
  (return (`/Game/Blueprints/Quest/Dialogues/BP_DialogueManager.IsStoryBlockActive` (`self.DialogueManagerRef`))))

(fn `RegisterDialogue`
  (params (Dialogue :type "/Game/Blueprints/Quest/Dialogues/Dialogue Structure"))
  (`/Game/Blueprints/Quest/Dialogues/BP_DialogueManager.RegisterDialogue` (`self.DialogueManagerRef`) Dialogue))

(fn `RegisterQuest`
  (params (Quest :type "/Game/Blueprints/Quest/BP_Quest Object Reference"))
  (if (not (`KismetArrayLibrary.Array_Contains` (`self.Quests`) Quest))
    (`KismetArrayLibrary.Array_Add` (`self.Quests`) Quest)))

(fn `RegisterStoryBlock`
  (params (Dialogue :type "/Game/Blueprints/Quest/Dialogues/Dialogue Structure"))
  (`/Game/Blueprints/Quest/Dialogues/BP_DialogueManager.RegisterStoryBlock` (`self.DialogueManagerRef`) Dialogue))

(fn `UserConstructionScript`)