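; Dialogue manager that shows character lines and story blocks through the player HUD widgets.
; Dialogue text is split at the colon into speaker and line, displayed, then hidden and marked done by a timer scaled to line length.
; Story blocks take their title field from the string table key and show the full text, with no auto-hide here.
; Query functions report whether dialogue is playing or a story block is visible.
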(event `RegisterDialogue`
  (params (Dialogue :type "/Game/Blueprints/Quest/Dialogues/Dialogue Structure"))
  (bind _id (break `/Game/Blueprints/Quest/Dialogues/Dialogue` Dialogue))
  (bind _dialoguewb (`self.DialogueWB`))
  (bind (_lefts _rights) (`KismetStringLibrary.Split` (`KismetTextLibrary.Conv_TextToString` _id) ":"))
  (bind _output_get (set `self.CurrentDialogue` (make `/Game/Blueprints/Quest/Dialogues/Dialogue` _id (`KismetStringLibrary.Conv_StringToName` _lefts) _rights)))
  (`/Game/Blueprints/Widgets/UI_Dialogue_WB.SetDialogue` _dialoguewb _output_get)
  (`/Game/Blueprints/Widgets/UI_Dialogue_WB.Show` _dialoguewb true)
  (`KismetSystemLibrary.K2_SetTimerDelegate` (delegate `EndDialogue`) (* (`KismetStringLibrary.Len` _rights) (`self.TimePerLetter`))))

(event `EndDialogue`
  (bind (_id _character _text) (break `/Game/Blueprints/Quest/Dialogues/Dialogue` (`self.CurrentDialogue`)))
  (set `self.CurrentDialogue` (make `/Game/Blueprints/Quest/Dialogues/Dialogue` _id _character _text true))
  (`/Game/Blueprints/Widgets/UI_Dialogue_WB.Show` (`self.DialogueWB`) false))

(event `RegisterStoryBlock`
  (params (Dialogue :type "/Game/Blueprints/Quest/Dialogues/Dialogue Structure"))
  (bind _id (break `/Game/Blueprints/Quest/Dialogues/Dialogue` Dialogue))
  (bind _storyblockwb (`self.StoryBlockWB`))
  (`/Game/Blueprints/Widgets/UI_StoryBlock_WB.SetStoryBlock` _storyblockwb (make `/Game/Blueprints/Quest/Dialogues/Dialogue` "" (`KismetStringLibrary.Conv_StringToName` (`.OutKey` (`KismetTextLibrary.StringTableIdAndKeyFromText` _id))) (`KismetTextLibrary.Conv_TextToString` _id)))
  (`/Game/Blueprints/Widgets/UI_StoryBlock_WB.Show` _storyblockwb true))

(fn `Init`
  (bind _hud (`/Game/Blueprints/BP_MiragePlayerController.Hud` (`/Game/Blueprints/BP_MirageLibrary.GetMiragePlayerController`)))
  (`parent.Init`)
  (set `self.DialogueWB` (`/Game/Blueprints/Widgets/UI_Hud.UI_Dialogue_WB` _hud))
  (set `self.StoryBlockWB` (`/Game/Blueprints/Widgets/UI_Hud.UI_StoryBlock_WB` _hud)))

(fn `IsPlaying`
  (returns (Playing :type Boolean))
  (return (not (`.Done_13_3120A8C34336EC026A7514A6E1576209` (break `/Game/Blueprints/Quest/Dialogues/Dialogue` (`self.CurrentDialogue`))))))

(fn `IsStoryBlockActive`
  (returns (Active :type Boolean))
  (return (`Widget.IsVisible` (`self.StoryBlockWB`))))

(fn `UserConstructionScript`)