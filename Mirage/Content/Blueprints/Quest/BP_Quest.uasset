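; BP_Quest is a quest Blueprint, likely a base for specific quests, that registers itself with the quest manager.
; On BeginPlay it fetches and caches the manager, registers if it is valid, then sets Started from ActiveOnStart.
; QShowHint and QHideHint forward to the manager's HintManager to show a hint by type or hide it, without validity checks.
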(event `self.ReceiveBeginPlay`
  (bind _output_get (set `self.QuestManagerRef` (`/Game/Blueprints/BP_MirageLibrary.GetQuestManager`)))
  (`/Engine/EditorBlueprintResources/StandardMacros.IsValid` _output_get
    (:`Is Valid`
      (`/Game/Blueprints/Quest/BP_QuestManager.RegisterQuest` (`self.QuestManagerRef`) self)
      (set `self.Started` (`self.ActiveOnStart`)))))

(fn `QHideHint`
  (`/Game/Blueprints/Hint/BP_HintManager.Hide` (`/Game/Blueprints/Quest/BP_QuestManager.HintManagerRef` (`self.QuestManagerRef`))))

(fn `QShowHint`
  (params (Type :type "/Game/Blueprints/Hint/HintType Enum" :default "NewEnumerator0"))
  (`/Game/Blueprints/Hint/BP_HintManager.Show` (`/Game/Blueprints/Quest/BP_QuestManager.HintManagerRef` (`self.QuestManagerRef`)) Type))

(fn `UserConstructionScript`)