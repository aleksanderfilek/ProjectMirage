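; BP_MirageGameMode is a game mode that creates and initializes the game's manager actors when play begins.
; SpawnManagers spawns each class key in the Managers map at the origin, owned by player controller 0, and stores the BP_Manager instance as that key's value.
; After a zero-length delay, it calls Init on every stored manager, so initialization runs only after spawning has finished.
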(event `self.ReceiveBeginPlay`
  (`|ExecutionSequence`
    (:`then_0`
      (`self.SpawnManagers`))
    (:`then_1`
      (`KismetSystemLibrary.Delay` 0.0)
      (bind _values (`BlueprintMapLibrary.Map_Values` (`self.Managers`)))
      (for _array_element _values
        (`/Game/Blueprints/BP_Manager.Init` _array_element)))))

(fn `SpawnManagers`
  (bind _keys (`BlueprintMapLibrary.Map_Keys` (`self.Managers`)))
  (for _array_element _keys
    (bind _returnvalue (`|SpawnActorFromClass` _array_element (`KismetMathLibrary.MakeTransform` (0.0 0.0 0.0)) "DontSpawnIfColliding" "OverrideRootScale" (`GameplayStatics.GetPlayerController` 0) null))
    (bind _asbp_manager (cast `/Game/Blueprints/BP_Manager` _returnvalue))
    (`BlueprintMapLibrary.Map_Add` (`self.Managers`) _array_element _asbp_manager)))

(fn `UserConstructionScript`)