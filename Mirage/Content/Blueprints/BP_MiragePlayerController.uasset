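; BP_MiragePlayerController is the Mirage player controller, managing the HUD and switching possession between a camera pawn and a character pawn.
; On BeginPlay it creates the HUD, shows the menu with UI-only input and a cursor in MainMenu, caches the controlled pawn as camera, and spawns the default character at the origin.
; Switch functions possess either pawn, with the character switch restoring game-only input.
; OnGameStarted reveals the crosshair.
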(event `self.ReceiveBeginPlay`
  (bind _playercontroller (`/Game/Blueprints/BP_MirageLibrary.GetMiragePlayerController`))
  (`|ExecutionSequence`
    (:`then_0`
      (bind _returnvalue (`|GenericCreateObject` "/Game/Blueprints/Widgets/UI_Hud.UI_Hud_C" self))
      (bind _output_get (set `self.Hud` _returnvalue))
      (`UserWidget.AddToViewport` _output_get -1)
      (bind _returnvalue_2 (`GameplayStatics.GetCurrentLevelName` true))
      (if (`KismetStringLibrary.EqualEqual_StrStr` _returnvalue_2 "MainMenu")
        (bind _returnvalue_3 (`|GenericCreateObject` "/Game/Blueprints/Widgets/UI_Menu_WB.UI_Menu_WB_C" self))
        (bind _output_get_2 (set `self.MenuWB` _returnvalue_3))
        (`UserWidget.AddToViewport` _output_get_2 0)
        (`WidgetBlueprintLibrary.SetInputMode_UIOnlyEx` _playercontroller (`self.MenuWB`))
        (set `PlayerController.bShowMouseCursor` true _playercontroller)))
    (:`then_1`
      (set `self.CameraPawnRef` (`self.K2_GetPawn`))
      (bind _returnvalue_4 (`|SpawnActorFromClass` "/Game/Blueprints/Characters/BP_MirageDefaultCharacter.BP_MirageDefaultCharacter_C" (`KismetMathLibrary.MakeTransform` (0.0 0.0 0.0)) "Undefined" "OverrideRootScale" null null))
      (set `self.CharacterPawnRef` _returnvalue_4))))

(event `Event On Game Started`
  (`Widget.SetVisibility` (`/Game/Blueprints/Widgets/UI_Hud.UI_Crosshair_WB` (`self.Hud`)) "Visible"))

(fn `SwitchPawnToCamera`
  (`self.Possess` (`self.CameraPawnRef`)))

(fn `SwitchPawnToCharacter`
  (`self.Possess` (`self.CharacterPawnRef`))
  (`WidgetBlueprintLibrary.SetInputMode_GameOnly` self)
  (set `self.bShowMouseCursor` false))

(fn `UserConstructionScript`)